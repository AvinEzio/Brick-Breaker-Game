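; Breakable box that loses one point of BoxStrength each time a Ball_BP hits it.
; Its cube material shows remaining strength as green, yellow or red, set on construction and after each non-fatal hit.
; At zero strength it explodes with sound and destroys itself.
; If no boxes remain, it reads LevelNo from LevelTracker_BP and shows the level-win widget, or the final win widget on level five.
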(event `self.ReceiveHit`
  (params (MyComp :type "PrimitiveComponent Object Reference") (Other :type "Actor Object Reference") (OtherComp :type "PrimitiveComponent Object Reference") (bSelfMoved :type Boolean) (HitLocation :type "Vector Structure") (HitNormal :type "Vector Structure") (NormalImpulse :type "Vector Structure") (Hit :type "HitResult Structure (by ref)"))
  (cast `/Game/Blueprints/Ball_BP` Other)
  (bind _result (`/Engine/EditorBlueprintResources/StandardMacros.DecrementInt` (`self.BoxStrength`))
    (:`  `
      (if (== _result 0)
        (`GameplayStatics.SpawnEmitterAtLocation` "/Game/StarterContent/Particles/P_Explosion.P_Explosion" (`self.K2_GetActorLocation`))
        (`GameplayStatics.PlaySoundAtLocation` "/Game/StarterContent/Audio/Explosion01.Explosion01" (`self.K2_GetActorLocation`) (struct) 1.0 1.0 0.0 null null null null)
        (`self.K2_DestroyActor`)
        (bind _outactors (`GameplayStatics.GetAllActorsOfClass` "Box_BP_C"))
        (if (== (`KismetArrayLibrary.Array_Length` _outactors) 0)
          (bind _returnvalue (`GameplayStatics.GetActorOfClass` "/Game/Blueprints/LevelTracker_BP.LevelTracker_BP_C"))
          (switch `int` (`/Game/Blueprints/LevelTracker_BP.LevelNo` _returnvalue)
            (:`1`
              (bind _returnvalue_2 (`|CreateWidget` "/Game/Blueprints/WinLevel_WB.WinLevel_WB_C"))
              (`UserWidget.AddToViewport` _returnvalue_2 0))
            (:`2`
              (bind _returnvalue_3 (`|CreateWidget` "/Game/Blueprints/WinLevel_WB.WinLevel_WB_C"))
              (`UserWidget.AddToViewport` _returnvalue_3 0))
            (:`3`
              (bind _returnvalue_4 (`|CreateWidget` "/Game/Blueprints/WinLevel_WB.WinLevel_WB_C"))
              (`UserWidget.AddToViewport` _returnvalue_4 0))
            (:`4`
              (bind _returnvalue_5 (`|CreateWidget` "/Game/Blueprints/WinLevel_WB.WinLevel_WB_C"))
              (`UserWidget.AddToViewport` _returnvalue_5 0))
            (:`5`
              (bind _returnvalue_6 (`|CreateWidget` "/Game/Blueprints/Win_WB.Win_WB_C"))
              (`UserWidget.AddToViewport` _returnvalue_6 0))))
        (else
          (`self.updateBoxColor`))))))

(fn `updateBoxColor`
  (bind _cube (`self.Cube`))
  (switch `int` (`self.BoxStrength`)
    (:`1`
      (`PrimitiveComponent.SetMaterial` _cube 0 "/Game/Materials/GreenGlow_Material1.GreenGlow_Material1"))
    (:`2`
      (`PrimitiveComponent.SetMaterial` _cube 0 "/Game/Materials/YellowGlow_Material.YellowGlow_Material"))
    (:`3`
      (`PrimitiveComponent.SetMaterial` _cube 0 "/Game/Materials/RedGlow_Material.RedGlow_Material"))))

(fn `UserConstructionScript`
  (`self.updateBoxColor`))