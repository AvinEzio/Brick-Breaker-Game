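; Physics-driven ball for a paddle game that bounces around at a steadily rising speed.
; BeginPlay launches it along X and caches the player's Paddle_BP.
; Each hit plays a beep, raises BallSpeed and locks velocity magnitude to it, updating the paddle HUD's score on "box"-tagged actors.
; On destruction it has the spawner create another ball while the paddle has lives, otherwise shows the Game Over widget.
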(event `self.ReceiveBeginPlay`
  (`PrimitiveComponent.AddImpulse` (`self.Sphere`) (1200.0 0.0 0.0) "None" true)
  (bind _aspaddle_bp (cast `/Game/Blueprints/Paddle_BP` (`GameplayStatics.GetPlayerPawn` 0)))
  (set `self.As Paddle BP` _aspaddle_bp))

(event `self.ReceiveHit`
  (params (MyComp :type "PrimitiveComponent Object Reference") (Other :type "Actor Object Reference") (OtherComp :type "PrimitiveComponent Object Reference") (bSelfMoved :type Boolean) (HitLocation :type "Vector Structure") (HitNormal :type "Vector Structure") (NormalImpulse :type "Vector Structure") (Hit :type "HitResult Structure (by ref)"))
  (bind _sphere (`self.Sphere`))
  (bind _ballspeed (`self.BallSpeed`))
  (`GameplayStatics.PlaySoundAtLocation` "/Game/Sound_Effects/ping_pong_8bit_beeep.ping_pong_8bit_beeep" (`self.K2_GetActorLocation`) (struct) 1.0 1.0 0.0 null null null null)
  (set `self.BallSpeed` (+ (`self.BallSpeed`) 2.0))
  (bind _returnvalue (`PrimitiveComponent.GetPhysicsLinearVelocity` _sphere "None"))
  (`PrimitiveComponent.SetPhysicsLinearVelocity` _sphere (`KismetMathLibrary.ClampVectorSize` _returnvalue _ballspeed _ballspeed) false "None")
  (if (`self.ActorHasTag` Other "box")
    (`/Game/Blueprints/HUD.Update Score` (`/Game/Blueprints/Paddle_BP.Player_HUD` (`self.As Paddle BP`)))))

(event `self.ReceiveDestroyed`
  (if (> (`/Game/Blueprints/Paddle_BP.Lives` (`self.As Paddle BP`)) 0)
    (`/Game/Blueprints/BallSpawner_BP.Spawn Ball` (`self.BallSpawnerRef`))
    (else
      (bind _returnvalue (`|CreateWidget` "/Game/Blueprints/GameOver_WB.GameOver_WB_C"))
      (`UserWidget.AddToViewport` _returnvalue 0))))

(fn `UserConstructionScript`)