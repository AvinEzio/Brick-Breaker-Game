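; Player paddle pawn for a ball game, moved along its vertical axis by player input.
; On BeginPlay it sets game-only input, adds the BallGame Enhanced Input mapping context and creates the player HUD.
; The move action offsets the Paddle component on Z with sweep, scaled by PaddleSpeed.
; Space Bar toggles pause, adding a new pause widget to the viewport when pausing.
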(event `self.ReceiveBeginPlay`
  (`WidgetBlueprintLibrary.SetInputMode_GameOnly` (`GameplayStatics.GetPlayerController` 0))
  (bind _asplayer_controller (cast `PlayerController` (`self.GetController`)))
  (bind _returnvalue (pcsubsystem `EnhancedInputLocalPlayerSubsystem` _asplayer_controller))
  (`/Engine/EditorBlueprintResources/StandardMacros.IsValid` _returnvalue
    (:`Is Valid`
      (`EnhancedInputSubsystemInterface.AddMappingContext` _returnvalue "/Game/Input/BallGame_IMC.BallGame_IMC" 0 (struct))
      (bind _returnvalue_2 (`|CreateWidget` "/Game/Blueprints/HUD.HUD_C"))
      (bind _output_get (set `self.Player_HUD` _returnvalue_2))
      (`UserWidget.AddToViewport` _output_get 0))))

(event `EnhancedInput|/Game/Input/Move_IA`
  (params (ActionValue :type "Float (double-precision)") (ElapsedSeconds :type "Float (double-precision)") (TriggeredSeconds :type "Float (double-precision)") (InputAction :type "InputAction Object Reference" :default "/Game/Input/Move_IA.Move_IA"))
  (:`Triggered`
    (`SceneComponent.K2_AddLocalOffset` (`self.Paddle`) (`KismetMathLibrary.MakeVector` 0.0 0.0 (* ActionValue (`self.PaddleSpeed`))) true false)))

(event `Key|SpaceBar` :paused true
  (params (Key :type "Key Structure"))
  (:`Pressed`
    (if (`GameplayStatics.IsGamePaused`)
      (`GameplayStatics.SetGamePaused` false)
      (else
        (`GameplayStatics.SetGamePaused` true)
        (bind _returnvalue (`|CreateWidget` "/Game/Blueprints/GamePause_WB.GamePause_WB_C"))
        (`UserWidget.AddToViewport` _returnvalue 0)))))

(fn `UserConstructionScript`)